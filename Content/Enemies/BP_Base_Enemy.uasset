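; Base enemy character with a sword melee attack, hit reactions and ragdoll death.
; Attack plays a montage whose notify applies damage via a sphere overlap, then fires OnAttackEnd when it finishes.
; Damage from Player-tagged causers lowers health, triggering a hit montage or death with delayed destruction.
; Exposes patrol route and movement speed functions; the looping ChasePlayer event has no active caller here.
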(event `self.ReceiveBeginPlay`)

(event `ChasePlayer`
  (`|AIMoveTo` self (0.0 0.0 0.0) (`GameplayStatics.GetPlayerCharacter` 0) 10.0
    (:`OnSuccess`
      (`self.Attack`)
      (`KismetSystemLibrary.Delay` 2.0)
      (`self.ChasePlayer`))))

(event `Attack`
  ;[0 0 0] Attack Event
  (`|PlayMontage` (`self.Mesh`) "/Game/Enemies/Skeleton/SwordMontage.SwordMontage"
    (:`OnCompleted`
      (`self.OnAttackEnd` :!label _label))
    (:`OnInterrupted`
      (goto _label))
    (:`OnNotifyBegin`
      (bind (_outactors _returnvalue) (`KismetSystemLibrary.SphereOverlapActors` (`SceneComponent.K2_GetComponentLocation` (`self.Arrow1`)) 100.0 (`|MakeArray` "ObjectTypeQuery1" "ObjectTypeQuery2" "ObjectTypeQuery3" :!type "EObjectTypeQuery Enum") null (`|MakeArray` self :!type "Actor Object Reference")))
      (if _returnvalue
        (for _array_element _outactors
          (`GameplayStatics.ApplyDamage` _array_element 15.0 null self "/Script/Engine.DamageType"))))))

(event `self.ReceiveAnyDamage`
  (params (Damage :type "Float (single-precision)") (DamageType :type "DamageType Object Reference") (InstigatedBy :type "Controller Object Reference") (DamageCauser :type "Actor Object Reference"))
  (bind _returnvalue (- (`self.Health`) Damage))
  ;[0 0 0] Take Damage Event
  (if (and (`self.ActorHasTag` DamageCauser "Player") (not (`self.isDead`)))
    (set `self.isAttacked` true)
    (if (<= _returnvalue 0.0)
      (set `self.Health` _returnvalue)
      (`KismetSystemLibrary.PrintString` "Dead")
      (`self.Enemy Death`)
      (else
        (set `self.Health` _returnvalue)
        (`|PlayMontage` (`self.Mesh`) "/Game/Enemies/Skeleton/CustomHitReactMontage.CustomHitReactMontage" 4.0
          (:`OnCompleted`
            _)
          (:`OnInterrupted`
            _))
        (set `self.isAttacked` false)))))

(event `Enemy Death`
  (bind _charactermovement (`self.CharacterMovement`))
  (set `self.isDead` true)
  (`PrimitiveComponent.SetSimulatePhysics` (`self.Mesh`) true)
  (`PrimitiveComponent.SetCollisionResponseToChannel` (`self.Mesh`) "ECC_Pawn" "ECR_Overlap")
  (`PrimitiveComponent.SetCollisionResponseToChannel` (`self.CapsuleComponent`) "ECC_Pawn" "ECR_Overlap")
  (`MovementComponent.StopMovementImmediately` _charactermovement)
  (`CharacterMovementComponent.DisableMovement` _charactermovement)
  (`KismetSystemLibrary.Delay` 10.0)
  (`self.K2_DestroyActor`))

(fn `GetPatrolRoute`
  (returns (PatrolRoute :type "/Game/Enemies/PatrolRouteSkeleton Object Reference"))
  (return (`self.PatrolRoute`)))

(fn `SetMovementSpeed`
  (params (Speed :type "/Game/Enemies/Enums/E_MovementSpeed Enum" :default "NewEnumerator0"))
  (returns (SpeedValue :type "Float (double-precision)"))
  (set `CharacterMovementComponent.MaxWalkSpeed` (select `/Game/Enemies/Enums/E_MovementSpeed` Speed :`NewEnumerator1` 150.0 :`NewEnumerator2` 500.0 :!type "Float (single-precision)") (`self.CharacterMovement`))
  (return 0.0))

(fn `UserConstructionScript`)