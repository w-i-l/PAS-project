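; Player pirate captain character with movement, mouse look, sword attack, health and save support.
; BeginPlay shows a timed loading screen, creates the HUD, starts a looping autosave and restores transform, health and control rotation through the GameInstance.
; Sword montage notifies trigger a sphere overlap that applies damage, while damage from Enemy-tagged actors updates the health bar and opens the death screen.
; Hotkeys handle manual saving, HUD toggling and the paused main menu.
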(event `self.ReceiveBeginPlay`
  (bind _returnvalue (`GameplayStatics.GetGameInstance`))
  ;[0 0 0] BeginPlay
  (`self.DisableInput` self (`GameplayStatics.GetPlayerController` 0))
  (bind _returnvalue_2 (`|CreateWidget` "/Game/UI/WB_LoadingScreen.WB_LoadingScreen_C"))
  (`UserWidget.AddToViewport` _returnvalue_2 0)
  (`KismetSystemLibrary.Delay` 3.0)
  (`Widget.RemoveFromParent` _returnvalue_2)
  (`self.EnableInput` self (`GameplayStatics.GetPlayerController` 0))
  (`self.SetupMainHUD`)
  (`KismetSystemLibrary.K2_SetTimerDelegate` (delegate `AutoSave`) 60.0 true)
  ;[0 0 0] Load Save
  (bind _asbp_game_instance (cast `/Game/SaveGame/BP_GameInstance` _returnvalue))
  (if (`/Game/SaveGame/BP_GameInstance.isGameSaved` _asbp_game_instance)
    (bind _savedgame (message `/Game/SaveGame/BPI_SaveGame.GetGameData` _returnvalue))
    (`/Engine/EditorBlueprintResources/StandardMacros.IsValid` _savedgame
      (:`Is Valid`
        (bind _returnvalue_3 (`GameplayStatics.GetActorOfClass` "BP_MyCharacter_C"))
        (`self.UsePlayerSave` _returnvalue_3 (`/Game/SaveGame/BP_SaveGame.PlayerSave` _savedgame))))))

(event `AutoSave`
  ;[0 0 0] AutoSave
  (bind _playersave (`self.GetPlayerSave`))
  (message `/Game/SaveGame/BPI_SaveGame.SavePlayer` (`GameplayStatics.GetGameInstance`) _playersave false))

(event `Key|Ctrl+E`
  (params (Key :type "Key Structure"))
  ;[0 0 0] Save Shortcut
  (:`Pressed`
    (`/Engine/EditorBlueprintResources/StandardMacros.DoOnce` false :!label _label
      (:`Completed`
        (if true
          (bind _playersave (`self.GetPlayerSave`))
          (message `/Game/SaveGame/BPI_SaveGame.SavePlayer` (`GameplayStatics.GetGameInstance`) _playersave false)
          (goto _label :!via `Reset`)))))
  (:`Released`
    (goto _label :!via `Reset`)))

(event `DeathEvent`
  (bind _returnvalue (`GameplayStatics.GetPlayerController` 0))
  ;[0 0 0] DeathEvent
  (bind _returnvalue_2 (`|CreateWidget` "/Game/UI/WB_Death.WB_Death_C"))
  (`UserWidget.AddToViewport` _returnvalue_2 0)
  (set `PlayerController.bShowMouseCursor` true _returnvalue)
  (`WidgetBlueprintLibrary.SetInputMode_UIOnlyEx` _returnvalue null)
  (`GameplayStatics.SetGamePaused` true))

(event `InputAxis|Move Forward / Backward`
  (params (AxisValue :type "Float (single-precision)"))
  (bind (_returnvalue_roll _returnvalue_pitch _returnvalue_yaw) (`KismetMathLibrary.BreakRotator` (`self.GetControlRotation`)))
  ;[0 0 0] Movement
  (`self.AddMovementInput` (`KismetMathLibrary.GetForwardVector` (`KismetMathLibrary.MakeRotator` _returnvalue_roll _returnvalue_pitch _returnvalue_yaw)) AxisValue))

(event `self.ReceiveAnyDamage`
  (params (Damage :type "Float (single-precision)") (DamageType :type "DamageType Object Reference") (InstigatedBy :type "Controller Object Reference") (DamageCauser :type "Actor Object Reference"))
  (bind _returnvalue (- (`self.Health`) Damage))
  ;[0 0 0] Event Receive Damage
  (if (and (`self.ActorHasTag` DamageCauser "Enemy") (not (`self.isDead`)))
    (if (<= (- (`self.Health`) Damage) 0.0)
      (set `self.Health` _returnvalue)
      (`self.DeathEvent`)
      (else
        (bind _output_get (set `self.Health` _returnvalue))
        (`KismetSystemLibrary.PrintString` (`KismetStringLibrary.Conv_DoubleToString` _output_get))))
    (`ProgressBar.SetPercent` (`/Game/UI/WB_MainHUD.HealthBar` (`self.MainHUDRef`)) (* (`self.Health`) 0.01))))

(event `InputAxis|Move Right / Left`
  (params (AxisValue :type "Float (single-precision)"))
  (bind (_returnvalue_roll _returnvalue_pitch _returnvalue_yaw) (`KismetMathLibrary.BreakRotator` (`self.GetControlRotation`)))
  ;[0 0 0] Movement
  (`self.AddMovementInput` (`KismetMathLibrary.GetRightVector` (`KismetMathLibrary.MakeRotator` _returnvalue_roll _returnvalue_pitch _returnvalue_yaw)) AxisValue))

(event `SetupMainHUD`
  ;[0 0 0] Create Main HUD
  (bind _returnvalue (`|CreateWidget` "/Game/UI/WB_MainHUD.WB_MainHUD_C" (`GameplayStatics.GetPlayerController` 0)))
  (bind _output_get (set `self.MainHUDRef` _returnvalue))
  (`UserWidget.AddToViewport` _output_get 0))

(event `InputAction|Jump`
  (params (Key :type "Key Structure"))
  ;[0 0 0] Movement
  (:`Pressed`
    (`self.Jump`)))

(event `Key|L`
  (params (Key :type "Key Structure"))
  (bind _mainhudref (`self.MainHUDRef`))
  ;[0 0 0] Show/Hide HUD
  (:`Pressed`
    (if (`self.isHudVisible`)
      (`Widget.SetVisibility` _mainhudref "Hidden")
      (set `self.isHudVisible` false)
      (else
        (`Widget.SetVisibility` _mainhudref "Visible")
        (set `self.isHudVisible` true)))))

(event `InputAxis|Look Up / Down Mouse`
  (params (AxisValue :type "Float (single-precision)"))
  ;[0 0 0] Camera
  (`self.AddControllerPitchInput` AxisValue))

(event `InputAxis|Turn Right / Left Mouse`
  (params (AxisValue :type "Float (single-precision)"))
  ;[0 0 0] Camera
  (`self.AddControllerYawInput` AxisValue))

(event `Key|LeftMouseButton`
  (params (Key :type "Key Structure"))
  ;[0 0 0] Attack Event
  (:`Pressed`
    (`/Engine/EditorBlueprintResources/StandardMacros.DoOnce` false :!label _label_2
      (:`Completed`
        (`|PlayMontage` (`self.Mesh`) "/Game/Characters/PirateCaptain/SwordMontage.SwordMontage"
          (:`OnCompleted`
            (`KismetSystemLibrary.Delay` 0.5)
            (goto _label_2 :!via `Reset`))
          (:`OnNotifyBegin`
            (bind (_outactors _returnvalue) (`KismetSystemLibrary.SphereOverlapActors` (`SceneComponent.K2_GetComponentLocation` (`self.Arrow1`)) 100.0 (`|MakeArray` "ObjectTypeQuery1" "ObjectTypeQuery2" "ObjectTypeQuery3" :!type "EObjectTypeQuery Enum") null (`|MakeArray` self :!type "Actor Object Reference")))
            (if _returnvalue
              (for _array_element _outactors
                (`GameplayStatics.ApplyDamage` _array_element 10.0 null self "/Script/Engine.DamageType")))))))))

(event `Key|M`
  (params (Key :type "Key Structure"))
  (bind _returnvalue (`GameplayStatics.GetPlayerController` 0))
  ;[0 0 0] MainMenuShortcut
  (:`Pressed`
    (bind _returnvalue_2 (`|CreateWidget` "/Game/UI/MainMenu.MainMenu_C"))
    (set `/Game/UI/MainMenu.isInGame` true _returnvalue_2)
    (`UserWidget.AddToViewport` _returnvalue_2 0)
    (set `PlayerController.bShowMouseCursor` true _returnvalue)
    (`WidgetBlueprintLibrary.SetInputMode_UIOnlyEx` _returnvalue null)
    (`GameplayStatics.SetGamePaused` true)))

(fn `GetPlayerSave`
  (returns (PlayerSave :type "/Game/SaveGame/S_PlayerSave Structure"))
  (return (make `/Game/SaveGame/S_PlayerSave` (`self.GetTransform`) (`self.Health`) (`self.GetControlRotation`))))

(fn `UsePlayerSave`
  (params (PlayerSave :type "/Game/SaveGame/S_PlayerSave Structure"))
  (if (not (== PlayerSave_Transform_2_832B2AD744A25122FBFCD483885F2440 (`KismetMathLibrary.MakeTransform` (0.0 0.0 0.0))))
    (`self.K2_SetActorTransform` PlayerSave_Transform_2_832B2AD744A25122FBFCD483885F2440)
    (set `self.Health` PlayerSave_Health_5_2D4164554E5A4D7D97DB84948858E7FC)
    (`Controller.SetControlRotation` (`self.GetController`) PlayerSave_ControlRotation_8_EE0D4DC4433200D0AF1610B19D876DE7)))

(fn `UserConstructionScript`)